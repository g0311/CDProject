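; BP_RSCharacter is a shooter AI character Blueprint that exposes combat stance events for its AI behavior.
; Cover crouches the character, while Retreat, Advance and Attack uncrouch it, with Attack followed by a half-second delay that leads to no further action.
; An UpdateWalkSpeed function sets the character movement component's maximum walk speed.
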(event EventAdvance
  (Character|UnCrouch))

(event Collision|EventActorBeginOverlap
  (params (OtherActor :type Actor%20Object%20Reference)))

(event EventTick
  (params (DeltaSeconds :type Float%20%28single-precision%29)))

(event EventRetreat
  (Character|UnCrouch))

(event EventAttack
  (Character|UnCrouch)
  (Utilities|FlowControl|Delay 0.5))

(event EventCover
  (Character|Crouch))

(fn ConstructionScript)

(fn UpdateWalkSpeed
  (params (New%20Walk%20Speed :type Float%20%28double-precision%29))
  (Variables|/Script/Engine.CharacterMovementComponent|SetMaxWalkSpeed (Variables|Character|GetCharacterMovement) New%20Walk%20Speed))