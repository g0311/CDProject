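; AI controller for deathmatch bots that runs BT_DeathMatch on possess and feeds it perception results through the Blackboard.
; Each perception update passes through sight, hearing and damage handlers, which filter by sense class.
; Sight and damage set TargetEnemy, or null it and store LastKnownLocation when the stimulus is lost; hearing stores HearingLocation.
; ExcuteDice writes a random DiceValue to the Blackboard, but nothing in this controller calls it.
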(event OnTargetPerceptionUpdated(AIPerception)
  (params (Actor :type Actor%20Object%20Reference) (Stimulus :type AI%20Stimulus%20Structure))
  (Variables|Default|SetSensedTarget Actor)
  (CallFunction|HandleSightSense Stimulus)
  (CallFunction|HandleSoundSense Stimulus)
  (CallFunction|HandleDamageSense Stimulus))

(event EventPossess
  (params (PossessedPawn :type Pawn%20Object%20Reference))
  (AI|RunBehaviorTree "/Game/BP/AI/DeathMatch/BT_DeathMatch.BT_DeathMatch"))

(fn ConstructionScript)

(fn HandleSoundSense
  (params (Stimulus :type AI%20Stimulus%20Structure))
  (bind _returnvalue (Class|AIPerceptionSystem|GetSenseClassforStimulus Stimulus))
  (if (== _returnvalue "/Script/AIModule.AISense_Hearing")
    ;[1 1 1] TargetLocation Set BlackBoard
    (AI|Components|Blackboard|SetValueasVector (Variables|Default|GetBlackboard) (Utilities|Name|MakeLiteralName "HearingLocation") (.StimulusLocation (Utilities|Struct|BreakAIStimulus Stimulus)))
    (Development|PrintString " HearingSense!")
    (else
      (return))))

(fn HandleSightSense
  (params (Stimulus :type AI%20Stimulus%20Structure))
  (bind _blackboard (Variables|Default|GetBlackboard))
  (bind _returnvalue (Class|AIPerceptionSystem|GetSenseClassforStimulus Stimulus))
  (if (== _returnvalue "/Script/AIModule.AISense_Sight")
    (AI|Components|Blackboard|SetValueasObject (Variables|Default|GetBlackboard) (Utilities|Name|MakeLiteralName "TargetEnemy") (Utilities|SelectObject (Variables|Default|GetSensedTarget) 0 (.bsuccessfullysensed Stimulus)))
    (if (.bsuccessfullysensed Stimulus)
      (Development|PrintString "SightOK")
      (else
        ;[1 1 1] If Lost Player
        (AI|Components|Blackboard|SetValueasVector _blackboard (Utilities|Name|MakeLiteralName "LastKnownLocation") (.stimuluslocation Stimulus))
        (AI|Components|Blackboard|ClearValue _blackboard (Utilities|Name|MakeLiteralName "TargetEnemy"))
        (Development|PrintString "SightLost")))
    (else
      (return))))

(fn HandleDamageSense
  (params (Stimulus :type AI%20Stimulus%20Structure))
  (bind _returnvalue (Class|AIPerceptionSystem|GetSenseClassforStimulus Stimulus))
  (if (== _returnvalue "/Script/AIModule.AISense_Damage")
    ;[1 1 1] Target Actor Player or Null
    (AI|Components|Blackboard|SetValueasObject (Variables|Default|GetBlackboard) (Utilities|Name|MakeLiteralName "TargetEnemy") (Utilities|SelectObject (Variables|Default|GetSensedTarget) 0 (.bsuccessfullysensed Stimulus)))
    (if (not (.bsuccessfullysensed Stimulus))
      ;[1 1 1] If Lost Player
      (AI|Components|Blackboard|SetValueasVector (Variables|Default|GetBlackboard) (Utilities|Name|MakeLiteralName "LastKnownLocation") (.stimuluslocation Stimulus)))
    (else
      (return))))

(fn ExcuteDice
  (bind _output_get (Variables|Default|SetDiceValue (Math|Random|RandomIntegerinRange 1 3)))
  (Class|BlackboardComponent|SetValueasInt (AI|GetBlackboard 0) (Utilities|Name|MakeLiteralName "DiceValue") _output_get))