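; AI controller for shooter bots that starts BB_Shooter2 on possess, seeding the blackboard with a random DiceValue and an IsDemolition flag.
; Perception updates cache target and own teams, then run sight, sound and damage handlers that write enemy and location keys.
; Sight filters by team but reads SensedTarget, whose assignment is unreachable.
; The damage handler tests the Sight sense and targets player 0 regardless of team.
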(event OnTargetPerceptionUpdated(AIPerception)
  (params (Actor :type Actor%20Object%20Reference) (Stimulus :type AI%20Stimulus%20Structure))
  ;[1 1 1] If Sensed Actor is Another Team -> Handle Sense
  (Utilities|FlowControl|Sequence
    (:then_0
      (bind _ascdcharacter (Utilities|Casting|CastToCDCharacter Actor))
      (Utilities|IsValid (Variables|/Script/Engine.Pawn|GetPlayerState _ascdcharacter)
        (:Is%20Valid
          (bind _ascdplayer_state (Utilities|Casting|CastToCDPlayerState (Variables|/Script/Engine.Pawn|GetPlayerState _ascdcharacter)))
          (Variables|Default|SetTargetTeam (Class|CDPlayerState|GetTeam _ascdplayer_state)))))
    (:then_1
      (bind _ascdcharacter_2 (Utilities|Casting|CastToCDCharacter (Pawn|GetControlledPawn)))
      (Utilities|IsValid (Variables|/Script/Engine.Pawn|GetPlayerState _ascdcharacter_2)
        (:Is%20Valid
          (bind _ascdplayer_state_2 (Utilities|Casting|CastToCDPlayerState (Variables|/Script/Engine.Pawn|GetPlayerState _ascdcharacter_2)))
          (Variables|Default|SetControlledTeam (Class|CDPlayerState|GetTeam _ascdplayer_state_2))))))
  (if true
    (CallFunction|HandleSightSense Stimulus)
    (CallFunction|HandleSoundSense Stimulus)
    (CallFunction|HandleDamageSense Stimulus)))

(event EventPossess
  (params (PossessedPawn :type Pawn%20Object%20Reference))
  ;[1 1 1] Set DiceValue && IsDemolition Mode?
  (CallFunction|ExcuteDice)
  (AI|RunBehaviorTree "/Game/BP/AI/AI_Info/BB_Shooter2.BB_Shooter2")
  (bind _asround_game_mode (Utilities|Casting|CastToRoundGameMode (Game|GetGameMode)))
  (Utilities|IsValid _asround_game_mode
    (:Is%20Valid
      (AI|Components|Blackboard|SetValueasBool (AI|GetBlackboard 0) (Utilities|Name|MakeLiteralName "IsDemolition") true))
    (:Is%20Not%20Valid
      (AI|Components|Blackboard|SetValueasBool (AI|GetBlackboard 0) (Utilities|Name|MakeLiteralName "IsDemolition") false))))

(fn ConstructionScript)

(fn HandleSoundSense
  (params (Stimulus :type AI%20Stimulus%20Structure))
  (bind _returnvalue (Class|AIPerceptionSystem|GetSenseClassforStimulus Stimulus))
  (if (== _returnvalue "/Script/AIModule.AISense_Hearing")
    ;[1 1 1] TargetLocation Set BlackBoard
    (AI|Components|Blackboard|SetValueasVector (Variables|Default|GetBlackboard) (Utilities|Name|MakeLiteralName "HearingLocation") (.StimulusLocation (Utilities|Struct|BreakAIStimulus Stimulus)))
    (Development|PrintString " HearingSense!")
    (else
      (return))))

(fn HandleSightSense
  (params (Stimulus :type AI%20Stimulus%20Structure))
  (bind _blackboard (Variables|Default|GetBlackboard))
  (bind _returnvalue (Class|AIPerceptionSystem|GetSenseClassforStimulus Stimulus))
  (if (== _returnvalue "/Script/AIModule.AISense_Sight")
    ;[1 1 1] Target Actor Player or Null
    (if (Utilities|Enum|NotEqual(Enum) (Variables|Default|GetTargetTeam) (Variables|Default|GetControlledTeam))
      (AI|Components|Blackboard|SetValueasObject (Variables|Default|GetBlackboard) (Utilities|Name|MakeLiteralName "TargetEnemy") (Utilities|SelectObject (Variables|Default|GetSensedTarget) 0 (.bsuccessfullysensed Stimulus)))
      (if (not (.bsuccessfullysensed Stimulus))
        ;[1 1 1] If Lost Player
        (AI|Components|Blackboard|SetValueasVector _blackboard (Utilities|Name|MakeLiteralName "LastKnownLocation") (.stimuluslocation Stimulus))
        (AI|Components|Blackboard|ClearValue _blackboard (Utilities|Name|MakeLiteralName "TargetEnemy"))
        (Development|PrintString "SightLost")))
    (else
      (return))))

(fn HandleDamageSense
  (params (Stimulus :type AI%20Stimulus%20Structure))
  (bind _returnvalue (Class|AIPerceptionSystem|GetSenseClassforStimulus Stimulus))
  (if (== _returnvalue "/Script/AIModule.AISense_Sight")
    ;[1 1 1] Target Actor Player or Null
    (AI|Components|Blackboard|SetValueasObject (Variables|Default|GetBlackboard) (Utilities|Name|MakeLiteralName "TargetEnemy") (Utilities|SelectObject (Game|GetPlayerCharacter 0) 0 (.bsuccessfullysensed Stimulus)))
    (if (not (.bsuccessfullysensed Stimulus))
      ;[1 1 1] If Lost Player
      (AI|Components|Blackboard|SetValueasVector (Variables|Default|GetBlackboard) (Utilities|Name|MakeLiteralName "LastKnownLocation") (.stimuluslocation Stimulus)))
    (else
      (return))))

(fn ExcuteDice
  (bind _output_get (Variables|Default|SetDiceValue (Math|Random|RandomIntegerinRange 1 3)))
  (Class|BlackboardComponent|SetValueasInt (AI|GetBlackboard 0) (Utilities|Name|MakeLiteralName "DiceValue") _output_get))