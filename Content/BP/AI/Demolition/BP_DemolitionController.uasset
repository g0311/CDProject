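; AI controller for bots in Demolition mode that runs BT_Demolition and feeds its blackboard.
; On possess it rolls a random DiceValue and sets IsDemolition when the game mode is a RoundGameMode.
; Perception updates compare CDPlayerState teams and pass other-team stimuli to sight, hearing and damage handlers.
; These handlers write TargetEnemy, HearingLocation and LastKnownLocation, recording where a target was lost.
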(event OnTargetPerceptionUpdated(AIPerception)
  (params (Actor :type Actor%20Object%20Reference) (Stimulus :type AI%20Stimulus%20Structure))
  ;[1 1 1] If Sensed Actor is Another Team -> Handle Sense
  (Variables|Default|SetSensedTarget Actor)
  (Utilities|FlowControl|Sequence
    (:then_0
      (bind _ascdcharacter (Utilities|Casting|CastToCDCharacter Actor))
      (Utilities|IsValid (Variables|/Script/Engine.Pawn|GetPlayerState _ascdcharacter)
        (:Is%20Valid
          (bind _ascdplayer_state (Utilities|Casting|CastToCDPlayerState (Variables|/Script/Engine.Pawn|GetPlayerState _ascdcharacter)))
          (Variables|Default|SetTargetTeam (Class|CDPlayerState|GetTeam _ascdplayer_state)))))
    (:then_1
      (bind _ascdcharacter_2 (Utilities|Casting|CastToCDCharacter (Pawn|GetControlledPawn)))
      (Utilities|IsValid (Variables|/Script/Engine.Pawn|GetPlayerState _ascdcharacter_2)
        (:Is%20Valid
          (bind _ascdplayer_state_2 (Utilities|Casting|CastToCDPlayerState (Variables|/Script/Engine.Pawn|GetPlayerState _ascdcharacter_2)))
          (Variables|Default|SetControlledTeam (Class|CDPlayerState|GetTeam _ascdplayer_state_2))
          (if (Utilities|Enum|NotEqual(Enum) (Class|CDPlayerState|GetTeam _ascdplayer_state) (Class|CDPlayerState|GetTeam _ascdplayer_state_2))
            (CallFunction|HandleSightSense Stimulus)
            (CallFunction|HandleSoundSense Stimulus)
            (CallFunction|HandleDamageSense Stimulus)))))))

(event EventPossess
  (params (PossessedPawn :type Pawn%20Object%20Reference))
  ;[1 1 1] Set DiceValue && IsDemolition Mode?
  (AI|RunBehaviorTree "/Game/BP/AI/Demolition/BT_Demolition.BT_Demolition")
  (CallFunction|ExcuteDice)
  (bind _asround_game_mode (Utilities|Casting|CastToRoundGameMode (Game|GetGameMode)))
  (Utilities|IsValid _asround_game_mode
    (:Is%20Valid
      (AI|Components|Blackboard|SetValueasBool (AI|GetBlackboard 0) (Utilities|Name|MakeLiteralName "IsDemolition") true))
    (:Is%20Not%20Valid
      (AI|Components|Blackboard|SetValueasBool (AI|GetBlackboard 0) (Utilities|Name|MakeLiteralName "IsDemolition") false))))

(fn ConstructionScript)

(fn HandleSoundSense
  (params (Stimulus :type AI%20Stimulus%20Structure))
  (bind _returnvalue (Class|AIPerceptionSystem|GetSenseClassforStimulus Stimulus))
  (if (== _returnvalue "/Script/AIModule.AISense_Hearing")
    ;[1 1 1] TargetLocation Set BlackBoard
    (AI|Components|Blackboard|SetValueasVector (Variables|Default|GetBlackboard) (Utilities|Name|MakeLiteralName "HearingLocation") (.StimulusLocation (Utilities|Struct|BreakAIStimulus Stimulus)))
    (Development|PrintString " HearingSense!")
    (else
      (return))))

(fn HandleSightSense
  (params (Stimulus :type AI%20Stimulus%20Structure))
  (bind _returnvalue (Utilities|Name|MakeLiteralName "TargetEnemy"))
  (bind _blackboard (Variables|Default|GetBlackboard))
  (bind _blackboard_2 (Variables|Default|GetBlackboard))
  (bind _returnvalue_2 (Class|AIPerceptionSystem|GetSenseClassforStimulus Stimulus))
  (if (== _returnvalue_2 "/Script/AIModule.AISense_Sight")
    ;[1 1 1] Target Actor Player or Null
    (if (!= (Variables|Default|GetTargetTeam) (Variables|Default|GetControlledTeam))
      (AI|Components|Blackboard|SetValueasObject _blackboard_2 _returnvalue (Utilities|SelectObject (Variables|Default|GetSensedTarget) 0 (.bsuccessfullysensed Stimulus)))
      (if (.bsuccessfullysensed Stimulus)
        (Development|PrintString "SightOK")
        (else
          ;[1 1 1] If Lost Player
          (AI|Components|Blackboard|SetValueasVector _blackboard (Utilities|Name|MakeLiteralName "LastKnownLocation") (.stimuluslocation Stimulus) :!label _label)
          (AI|Components|Blackboard|ClearValue _blackboard (Utilities|Name|MakeLiteralName "TargetEnemy"))
          (Development|PrintString "SightLost")))
      (else
        (AI|Components|Blackboard|SetValueasObject _blackboard_2 _returnvalue 0)
        (goto _label)))
    (else
      (return))))

(fn HandleDamageSense
  (params (Stimulus :type AI%20Stimulus%20Structure))
  (bind _returnvalue (Class|AIPerceptionSystem|GetSenseClassforStimulus Stimulus))
  (if (== _returnvalue "/Script/AIModule.AISense_Damage")
    ;[1 1 1] Target Actor Player or Null
    (AI|Components|Blackboard|SetValueasObject (Variables|Default|GetBlackboard) (Utilities|Name|MakeLiteralName "TargetEnemy") (Utilities|SelectObject (Variables|Default|GetSensedTarget) 0 (.bsuccessfullysensed Stimulus)))
    (if (not (.bsuccessfullysensed Stimulus))
      ;[1 1 1] If Lost Player
      (AI|Components|Blackboard|SetValueasVector (Variables|Default|GetBlackboard) (Utilities|Name|MakeLiteralName "LastKnownLocation") (.stimuluslocation Stimulus)))
    (else
      (return))))

(fn ExcuteDice
  (bind _output_get (Variables|Default|SetDiceValue (Math|Random|RandomIntegerinRange 1 3)))
  (Class|BlackboardComponent|SetValueasInt (AI|GetBlackboard 0) (Utilities|Name|MakeLiteralName "DiceValue") _output_get))